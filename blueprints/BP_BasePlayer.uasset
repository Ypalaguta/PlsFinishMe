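; BP_BasePlayer is a base player Blueprint providing HUD setup and inventory initialization for what appears to be an RPG.
; Init functions create UI widgets (bars, chat, inventory, death screen, actions), pass them the player and add them to the viewport.
; Inventory setup spawns hardcoded BP_Item actors, then pads inventory and equipment slots, leaving JSON item loading disconnected.
; UI, respawn, message and inventory trigger events are print-only stubs.
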(event Custom|triggerInventoryItemDblClick
  (params (item :type BP%20Item%20Object%20Reference))
  (Development|PrintString "inventoryDrop"))

(event Custom|triggerUIOther
  (Development|PrintString "triggerUITeleport"))

(event Custom|triggerUIInventory
  (Development|PrintString "triggerUITeleport"))

(event Custom|triggerUISkills
  (Development|PrintString "triggerUITeleport"))

(event Custom|triggerRespawn
  (Development|PrintString "respawn"))

(event Custom|triggerUIMap
  (Development|PrintString "triggerUITeleport"))

(event Custom|triggerMessage
  (Development|PrintString "message"))

(event Custom|triggerUITeleport
  (Development|PrintString "triggerUITeleport"))

(event Custom|triggerUIQuest
  (Development|PrintString "triggerUITeleport"))

(event Custom|triggerInventoryDrop
  (params (dragSlotNum :type Integer) (dropSlotNum :type Integer))
  (Development|PrintString "inventoryDrop"))

(event Custom|triggerUICharacterInfo
  (Development|PrintString "triggerUITeleport"))

(event EventBeginPlay)

(event Collision|EventActorBeginOverlap
  (params (OtherActor :type Actor%20Object%20Reference)))

(event EventTick
  (params (DeltaSeconds :type Float%20%28single-precision%29)))

(fn ConstructionScript)

(fn InitWBPCharacterBars
  (bind _returnvalue (UserInterface|CreateWidget "/Game/0Main/widgets/WBP_CharacterBars.WBP_CharacterBars_C" (Game|GetPlayerController 0)))
  (bind _output_get (Variables|Default|SetWBP_CharacterBars _returnvalue))
  (Default|InitRefs _output_get self)
  (UserInterface|Viewport|AddtoViewport _output_get 0))

(fn InitWBPSkillsBar
  (bind _returnvalue (UserInterface|CreateWidget "/Game/0Main/widgets/WBP_SkillsBar.WBP_SkillsBar_C" (Game|GetPlayerController 0)))
  (bind _output_get (Variables|Default|SetWBP_SkillsBar _returnvalue))
  (Default|InitRefs _output_get self)
  (UserInterface|Viewport|AddtoViewport _output_get 0))

(fn InitWBPChat
  (bind _returnvalue (UserInterface|CreateWidget "/Game/0Main/widgets/WBP_Chat/WBP_Chat.WBP_Chat_C" (Game|GetPlayerController 0)))
  (bind _output_get (Variables|Default|SetWBP_Chat _returnvalue))
  (Default|InitRefs _output_get self)
  (UserInterface|Viewport|AddtoViewport _output_get 0))

(fn InitSlotKeyAssignments
  (Class|VaRestSubsystem|LoadJsonfromFile (|VaRestSubsystem) "" true))

(fn InitWBPDeadScreen
  (bind _returnvalue (UserInterface|CreateWidget "/Game/0Main/widgets/WBP_DeadScreen.WBP_DeadScreen_C" (Game|GetPlayerController 0)))
  (bind _output_get (Variables|Default|SetWBP_DeadScreen _returnvalue))
  (Default|InitRefs _output_get self)
  (UserInterface|Viewport|AddtoViewport _output_get 0))

(fn InitWBPSkillUseProgressBar
  (bind _returnvalue (UserInterface|CreateWidget "/Game/0Main/widgets/WBP_SkillUseProgressBar.WBP_SkillUseProgressBar_C" (Game|GetPlayerController 0)))
  (bind _output_get (Variables|Default|SetWBP_SkillUseProgressBar _returnvalue))
  (Default|InitRefs _output_get self)
  (UserInterface|Viewport|AddtoViewport _output_get 0))

(fn InitWBPActionsUI
  (bind _returnvalue (UserInterface|CreateWidget "/Game/0Main/widgets/WBP_ActionsUI.WBP_ActionsUI_C" (Game|GetPlayerController 0)))
  (bind _output_get (Variables|Default|SetWBP_ActionsUI _returnvalue))
  (Default|InitRefs _output_get self)
  (UserInterface|Viewport|AddtoViewport _output_get 0))

(fn InitWBPInventory
  (bind _returnvalue (Game|GetPlayerController 0))
  (Utilities|FlowControl|Sequence
    (:then_0
      (bind _returnvalue_2 (UserInterface|CreateWidget "/Game/0Main/widgets/WBP_Inventory/WBP_Inventory.WBP_Inventory_C" _returnvalue))
      (bind _output_get (Variables|Default|SetWBP_Inventory _returnvalue_2))
      (Default|InitRefs _output_get self _returnvalue)
      (UserInterface|Viewport|AddtoViewport _output_get 0))))

(fn InitInventoryItems
  (bind _self self)
  (bind _self_2 self)
  (bind _self_3 self)
  (bind _self_4 self)
  (bind _inventory (Variables|Default|Getinventory))
  (bind _index (LocalVariables|Getindex))
  (bind _temptypes (LocalVariables|GettempTypes))
  (bind _temptypes_2 (LocalVariables|GettempTypes))
  (bind _temptypes_3 (LocalVariables|GettempTypes))
  (bind _temptypes_4 (LocalVariables|GettempTypes))
  (Utilities|FlowControl|Sequence
    (:then_0
      (Utilities|FlowControl|Sequence
        (:then_0
          (bind _returnvalue (Game|SpawnActorfromClass "/Game/0Main/blueprints/BP_Item.BP_Item_C" (Math|Transform|MakeTransform (LocalVariables|GetitemLoc) "0, 0, 0" "1.000000,1.000000,1.000000") "Undefined" "MultiplyWithRoot" _self _self))
          (Utilities|Array|Clear _temptypes_4)
          (Utilities|Array|Add _temptypes_4 "NewEnumerator28")
          (Default|Init _returnvalue (LocalVariables|GettempTypes) 1 "/Game/0Main/Assets/Image/Icons/R_Gold.R_Gold" 500)
          (Utilities|Array|Add (Variables|Default|Getinventory) _returnvalue))
        (:then_1
          (bind _returnvalue_2 (Game|SpawnActorfromClass "/Game/0Main/blueprints/BP_Item.BP_Item_C" (Math|Transform|MakeTransform (LocalVariables|GetitemLoc) "0, 0, 0" "1.000000,1.000000,1.000000") "Undefined" "MultiplyWithRoot" _self_3 _self_3))
          (Utilities|Array|Clear _temptypes_3)
          (Utilities|Array|Add _temptypes_3 "NewEnumerator2")
          (Default|Init _returnvalue_2 (LocalVariables|GettempTypes) 2)
          (Utilities|Array|Add (Variables|Default|Getinventory) _returnvalue_2))
        (:then_2
          (bind _returnvalue_3 (Game|SpawnActorfromClass "/Game/0Main/blueprints/BP_Item.BP_Item_C" (Math|Transform|MakeTransform (LocalVariables|GetitemLoc) "0, 0, 0" "1.000000,1.000000,1.000000") "Undefined" "MultiplyWithRoot" _self_4 _self_4))
          (Utilities|Array|Clear _temptypes_2)
          (Utilities|Array|Add _temptypes_2 "NewEnumerator2")
          (Default|Init _returnvalue_3 (LocalVariables|GettempTypes) 3)
          (Utilities|Array|Add (Variables|Default|Getinventory) _returnvalue_3))
        (:then_3
          (bind _returnvalue_4 (Game|SpawnActorfromClass "/Game/0Main/blueprints/BP_Item.BP_Item_C" (Math|Transform|MakeTransform (LocalVariables|GetitemLoc) "0, 0, 0" "1.000000,1.000000,1.000000") "Undefined" "MultiplyWithRoot" _self_2 _self_2))
          (Utilities|Array|Clear _temptypes)
          (Utilities|Array|Add _temptypes "NewEnumerator14")
          (Default|Init _returnvalue_4 (LocalVariables|GettempTypes) 4)
          (Utilities|Array|Add (Variables|Default|Getinventory) _returnvalue_4))))
    (:then_1
      (while (< (Utilities|Array|Length _inventory) (Variables|/Game/0Main/blueprints/BP_CharacterInfo.BP_CharacterInfo_C|GetbonusInventorySlots (Variables|Default|GetBP_CharacterInfo)))
        (Utilities|Array|Add _inventory 0)))
    (:then_3
      (while (< _index 17)
        (Utilities|Array|Add (Variables|Default|GetequippedItems) 0)
        (Math|Integer|IncrementInt _index)))))