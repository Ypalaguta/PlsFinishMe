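; Base character Blueprint holding skill data and helper functions for characters, including players.
; Helpers find and update Skills entries by Id, reverse-look up a slot from its key in SlotKeyAssignments, and destroy the actor.
; UseSkillUI casts self to BP_BasePlayer to drive its skill-use progress bar with time, icon and name.
; UseSkill and MakeCharacterSkill are empty stubs, and the event graph is inactive.
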(event EventBeginPlay)

(event Collision|EventActorBeginOverlap
  (params (OtherActor :type Actor%20Object%20Reference)))

(event EventTick
  (params (DeltaSeconds :type Float%20%28single-precision%29)))

(fn ConstructionScript)

(fn Destroy
  (Actor|DestroyActor))

(fn GetSlotbyKey
  (params (key :type String))
  (bind _slotkeyassignments (Variables|dataMaps|GetslotKeyAssignments))
  (bind _keys (Utilities|Map|Keys _slotkeyassignments))
  (for _array_element _keys
    (if (Utilities|Enum|Equal(Enum) key (.Value (Utilities|Map|Find _slotkeyassignments _array_element)))
      (return _array_element)))
  (return (LocalVariables|GetnotFound)))

(fn UpdCharacterSkill
  (params (skill :type S%20Skill%20Structure))
  (bind _skills (Variables|dataMaps|Getskills))
  (for (_array_element _array_index) _skills
    (if (== (Utilities|Struct|BreakS_Skill _array_element) (Utilities|Struct|BreakS_Skill skill))
      (Utilities|Array|SetArrayElem _skills _array_index skill))))

(fn MakeCharacterSkill
  (return ""))

(fn UseSkillUI
  (params (skill :type S%20Skill%20Structure))
  (bind (_usetime _icon _displayname) (Utilities|Struct|BreakS_Skill skill))
  (bind _asbp_base_player (Utilities|Casting|CastToBP_BasePlayer self))
  (Default|UseSkill (Variables|/Game/0Main/blueprints/BP_BasePlayer.BP_BasePlayer_C|GetWBP_SkillUseProgressBar _asbp_base_player) _usetime (.Value (Utilities|Map|Find (Variables|staticData|GetskillIcons) _icon)) _displayname))

(fn GetSkillbyId
  (params (id :type Integer))
  (for (_array_element _array_index) (Variables|dataMaps|Getskills)
    (if (== (Utilities|Struct|BreakS_Skill _array_element) id)
      (return _array_element _array_index))))

(fn UseSkill
  (params (skillId :type Integer)))