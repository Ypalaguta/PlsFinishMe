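; Manages persistent BP_BaseEnemy spawn points, storing location, death state and respawn time in a JSON file.
; Init loads records via VaRest, spawning enemies with offset-based patrol coordinates.
; CreatureDied stamps a Unix respawn time; CheckSpawns runs on a repeating timer, respawning due enemies and saving to a hardcoded absolute path.
; SwawnCreature adds a spawn at the player; RemoveCreature parses a command ID to destroy and unregister one.
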(event EventBeginPlay
  (CallFunction|Init)
  (CallFunction|CheckSpawns))

(event Collision|EventActorBeginOverlap
  (params (OtherActor :type Actor%20Object%20Reference)))

(event EventTick
  (params (DeltaSeconds :type Float%20%28single-precision%29)))

(fn ConstructionScript)

(fn SwawnCreature
  (params (command :type String))
  (bind _returnvalue (Game|Player|GetPlayerPawn 0))
  (bind _returnvalue_2 (Transformation|GetActorLocation _returnvalue))
  (Utilities|FlowControl|Sequence
    (:then_0
      (bind _res (CallFunction|GetIdtoSet))
      (LocalVariables|SetidToSet _res))
    (:then_1
      (bind _structout (Utilities|Struct|SetmembersinS_Spawn (LocalVariables|GetNewLocalVar) _returnvalue_2 10 (LocalVariables|GetidToSet)))
      (Utilities|Array|Add (Variables|Default|Getspawns) _structout)
      (CallFunction|Save))
    (:then_2
      (bind _returnvalue_3 (Game|SpawnActorfromClass "/Game/0Main/Characters/BaseEnemy/BP_BaseEnemy.BP_BaseEnemy_C" (Math|Transform|MakeTransform (+ (* (Transformation|GetActorForwardVector _returnvalue) (LocalVariables|GetforwardMultiplier)) _returnvalue_2) "0, 0, 0" "1.000000,1.000000,1.000000") "AdjustIfPossibleButAlwaysSpawn" "MultiplyWithRoot" 0 0))
      (Variables|/Game/0Main/Characters/Manny/BP_BaseCharacter.BP_BaseCharacter_C|SetspawnId _returnvalue_3 (LocalVariables|GetidToSet)))))

(fn Init
  (bind _tempspawnstruct (LocalVariables|GettempSpawnStruct))
  (bind _tempspawnstruct_2 (LocalVariables|GettempSpawnStruct))
  (bind _patroloffsetcoords (LocalVariables|GetpatrolOffsetCoords))
  (bind (_enemyid _location _isdead _respawnat _respawntime _id) (Utilities|Struct|BreakS_Spawn _tempspawnstruct))
  (Development|PrintString "spawn 0")
  (bind _returnvalue (Class|VaRestSubsystem|LoadJsonfromFile (|VaRestSubsystem) (Variables|Default|GetPath) true))
  (Utilities|IsValid _returnvalue
    (:Is%20Valid
      (Utilities|IsValid (Class|VaRestJsonObject|GetField _returnvalue "items")
        (:Is%20Valid
          (for _array_element (Class|VaRestJsonValue|AsArray (Class|VaRestJsonObject|GetField _returnvalue "items"))
            (bind _returnvalue_2 (Class|VaRestJsonValue|AsObject _array_element))
            (for _array_element_2 (Class|VaRestJsonObject|GetFieldNames _returnvalue_2)
              (switch string _array_element_2
                (:Default
                  (Development|PrintString "unidentified field found on spawn data load"))
                (:id
                  (Utilities|Struct|SetmembersinS_Spawn _tempspawnstruct_2 (Class|VaRestJsonValue|AsInt32 (Class|VaRestJsonObject|GetField _returnvalue_2 _array_element_2))))
                (:enemyId
                  (Utilities|Struct|SetmembersinS_Spawn _tempspawnstruct_2 (Class|VaRestJsonValue|AsInt32 (Class|VaRestJsonObject|GetField _returnvalue_2 _array_element_2))))
                (:location
                  (bind _returnvalue_3 (Class|VaRestJsonValue|AsObject (Class|VaRestJsonObject|GetField _returnvalue_2 _array_element_2)))
                  (Utilities|Struct|SetmembersinS_Spawn _tempspawnstruct_2 (Math|Vector|MakeVector (Class|VaRestJsonValue|AsNumber (Class|VaRestJsonObject|GetField _returnvalue_3 "x")) (Class|VaRestJsonValue|AsNumber (Class|VaRestJsonObject|GetField _returnvalue_3 "y")) (Class|VaRestJsonValue|AsNumber (Class|VaRestJsonObject|GetField _returnvalue_3 "z")))))
                (:isDead
                  (Utilities|Struct|SetmembersinS_Spawn _tempspawnstruct_2 (Class|VaRestJsonValue|AsBool (Class|VaRestJsonObject|GetField _returnvalue_2 _array_element_2))))
                (:respawnAt
                  (Utilities|Struct|SetmembersinS_Spawn _tempspawnstruct_2 (Class|VaRestJsonValue|AsNumber (Class|VaRestJsonObject|GetField _returnvalue_2 _array_element_2))))
                (:respawnTime
                  (Utilities|Struct|SetmembersinS_Spawn _tempspawnstruct_2 (Class|VaRestJsonValue|AsInt32 (Class|VaRestJsonObject|GetField _returnvalue_2 _array_element_2))))))
            (Utilities|Array|Add (Variables|Default|Getspawns) (|Copy _tempspawnstruct))
            (bind _returnvalue_4 (Game|SpawnActorfromClass "/Game/0Main/Characters/BaseEnemy/BP_BaseEnemy.BP_BaseEnemy_C" (Math|Transform|MakeTransform _location "0, 0, 0" "1.000000,1.000000,1.000000") "Undefined" "MultiplyWithRoot" 0 0))
            (Variables|/Game/0Main/Characters/Manny/BP_BaseCharacter.BP_BaseCharacter_C|SetspawnId _returnvalue_4 _id)
            (for _array_element_3 (LocalVariables|GetpatrolOffset)
              (Utilities|Array|Add _patroloffsetcoords (+ _array_element_3 _location)))
            (Utilities|Array|Add _patroloffsetcoords _location)
            (Variables|/Game/0Main/Characters/BaseEnemy/BP_BaseEnemy.BP_BaseEnemy_C|SetpatrolCoords _returnvalue_4 _patroloffsetcoords)
            (Development|PrintString (Utilities|String|Append "setting spawned enemy patrol coords " (Utilities|String|ToString(Vector) (Utilities|Array|Get(acopy) _patroloffsetcoords)) " | " (Utilities|String|ToString(Vector) (Utilities|Array|Get(acopy) _patroloffsetcoords 1)) " | " (Utilities|String|ToString(Vector) (Utilities|Array|Get(acopy) _patroloffsetcoords 2)) " | " (Utilities|String|ToString(Vector) (Utilities|Array|Get(acopy) _patroloffsetcoords 3))))
            (Default|PatrolSet _returnvalue_4)))))))

(fn Save
  (for (_array_element _array_index) (Variables|Default|Getspawns)
    (bind _outjsonstring (|StructtoJsonString _array_element))
    (if (== _array_index 0)
      (Variables|Default|SetconvertedStructs _outjsonstring)
      (else
        (Variables|Default|SetconvertedStructs (Utilities|String|Append (Variables|Default|GetconvertedStructs) "," _outjsonstring)))))
  (bind _output_get (Variables|Default|SetjsonRes (Utilities|String|Append "{ 
   \"items\":[" (Variables|Default|GetconvertedStructs) "   ] 
}")))
  (Class|FileSDKBPLibrary|WriteStringtoFile "F:\\tempunrealprojects\\NewWorld\\Content\\0Main\\Mock\\spawn.json" _output_get false "AutoDetect"))

(fn CheckSpawns
  (bind _returnvalue (Math|DateTime|Now))
  (bind _spawns (Variables|Default|Getspawns))
  (bind _returnvalue_2 (Class|KismetMathLibrary|ToUnixTimestamp _returnvalue))
  (for (_array_element _array_index) _spawns
    (Development|PrintString (Utilities|String|Append "check spawns now " (Utilities|String|ToString(Integer) _returnvalue_2) "| resp at |" (Utilities|String|ToString(Float) (.respawnAt (Utilities|Struct|BreakS_Spawn _array_element))) "id = " (Utilities|String|ToString(Integer) (.id (Utilities|Struct|BreakS_Spawn _array_element)))))
    (if (and (> _returnvalue_2 (.respawnAt (Utilities|Struct|BreakS_Spawn _array_element))) (.isDead (Utilities|Struct|BreakS_Spawn _array_element)))
      (bind _returnvalue_3 (Game|SpawnActorfromClass "/Game/0Main/Characters/BaseEnemy/BP_BaseEnemy.BP_BaseEnemy_C" (Math|Transform|MakeTransform (.location (Utilities|Struct|BreakS_Spawn _array_element)) "0, 0, 0" "1.000000,1.000000,1.000000") "AdjustIfPossibleButAlwaysSpawn" "MultiplyWithRoot" 0 0))
      (Variables|/Game/0Main/Characters/Manny/BP_BaseCharacter.BP_BaseCharacter_C|SetspawnId _returnvalue_3 (.id (Utilities|Struct|BreakS_Spawn _array_element)))
      (bind _structout (Utilities|Struct|SetmembersinS_Spawn _array_element false 0.0))
      (Utilities|Array|SetArrayElem _spawns _array_index _structout)))
  (CallFunction|Save)
  (Utilities|Time|SetTimerbyFunctionName 0 "checkSpawns" 1e+01))

(fn GetIdtoSet
  (for _array_element (Variables|Default|Getspawns)
    (if (> (.id (Utilities|Struct|BreakS_Spawn _array_element)) (LocalVariables|GetidToSet))
      (LocalVariables|SetidToSet (.id (Utilities|Struct|BreakS_Spawn _array_element)))))
  (return (+ (LocalVariables|GetidToSet) 1)))

(fn CreatureDied
  (params (spawnId :type Integer))
  (bind _spawns (Variables|Default|Getspawns))
  (Development|PrintString (Utilities|String|Append "creatureDied | " (Utilities|String|ToString(Integer) spawnId)))
  (for (_array_element _array_index) _spawns
    (if (== (.id (Utilities|Struct|BreakS_Spawn _array_element)) spawnId)
      (bind _structout (Utilities|Struct|SetmembersinS_Spawn _array_element true (Math|Conversions|ToFloat(Integer) (+ (Class|KismetMathLibrary|ToUnixTimestamp (Math|DateTime|Now)) (.respawnTime (Utilities|Struct|BreakS_Spawn _array_element))))))
      (Utilities|Array|SetArrayElem _spawns _array_index _structout))))

(fn RemoveCreature
  (params (command :type String))
  (bind _newparam (CallFunction|GetCmdParams command))
  (bind _isvalid (CallFunction|IsStrValidtoInt (Utilities|Array|Get(acopy) _newparam 1)))
  (if _isvalid
    (Development|PrintString "/despawn 1")
    (Utilities|FlowControl|Sequence
      (:then_0
        (bind _outactors (Actor|GetAllActorsOfClass "/Game/0Main/Characters/BaseEnemy/BP_BaseEnemy.BP_BaseEnemy_C"))
        (for _array_element _outactors
          (if (== (Variables|/Game/0Main/Characters/Manny/BP_BaseCharacter.BP_BaseCharacter_C|GetspawnId _array_element) (Math|Conversions|ToInteger(Byte) (Utilities|Array|Get(acopy) _newparam 1)))
            (Actor|DestroyActor _array_element)))
        (Development|PrintString "/despawn 2")
        (bind _status (CallFunction|RemovefromSpawn (Math|Conversions|ToInteger(Byte) (Utilities|Array|Get(acopy) _newparam 1))))
        (if _status
          (CallFunction|Save)
          (Development|PrintString "/despawn 3")
          (else
            (Development|PrintString "/despawn remove element error")))))
    (else
      (Development|PrintString "Hello"))))

(fn GetCmdParams
  (params (command :type String))
  (return (Utilities|String|ParseIntoArray command (LocalVariables|Getspace))))

(fn IsStrValidtoInt
  (params (str :type String))
  (return (not (and (== (Math|Conversions|ToInteger(Byte) str) 0) (not (Utilities|Enum|Equal(Enum) str "0"))))))

(fn RemovefromSpawn
  (params (id :type Integer))
  (bind _spawns (Variables|Default|Getspawns))
  (bind (_array_element _array_index) (Utilities|Array|ForEachLoopwithBreak _spawns)
    (:LoopBody
      (if (== (Utilities|Struct|BreakS_Spawn _array_element) id)
        (Utilities|Array|RemoveIndex _spawns _array_index)
        (return true)))
    (:Completed
      (return true))))